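; AI-controlled player that slides its Cube along X to follow the Ball actor, like an automated paddle.
; BeginPlay sets the tick interval; each tick looks up the Ball, stores its Sphere's relative location and calls Move.
; Move uses MoveComponentTo over MovingTime toward the clamped ball X, feeding the Cube's world Y, Z and rotation into the relative-space target.
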(event Custom|Move
  (bind _cube (Variables|Default|GetCube))
  (bind _returnvalue (Transformation|GetWorldTransform _cube))
  (Components|MoveComponentTo _cube (Math|Vector|MakeVector (Math|Float|Clamp(Float) (.x (Variables|Default|GetBall_Loc)) -3.1e+02 3.1e+02) (.y (.location _returnvalue)) (.z (.location _returnvalue))) (.rotation _returnvalue) false false (Variables|Default|GetMovingTime) false))

(event EventBeginPlay
  (Actor|Tick|SetActorTickInterval (Variables|Default|GetTick%20Interval)))

(event Collision|EventActorBeginOverlap
  (params (OtherActor :type Actor%20Object%20Reference)))

(event EventTick
  (params (DeltaSeconds :type Float%20%28single-precision%29))
  (bind _returnvalue (Actor|GetActorOfClass "/Game/BluePrints/Ball.Ball_C"))
  (Variables|Default|SetBall_Loc (Math|Vector|MakeVector (.x (Variables|/Script/Engine.SceneComponent|GetRelativeLocation (Variables|/Game/BluePrints/Ball.Ball_C|GetSphere _returnvalue))) (.y (Variables|/Script/Engine.SceneComponent|GetRelativeLocation (Variables|/Game/BluePrints/Ball.Ball_C|GetSphere _returnvalue))) (.z (Variables|/Script/Engine.SceneComponent|GetRelativeLocation (Variables|/Game/BluePrints/Ball.Ball_C|GetSphere _returnvalue)))))
  (CallFunction|Move))

(fn ConstructionScript)