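; Player pawn that slides its Cube component along local X from axis input and puts the ScorePanel widget on screen at BeginPlay.
; Each Tick scales the axis value, clamps it between MinValue and MaxValue and applies it as a local offset, without delta-time scaling.
; ChangingSpeed overwrites both clamp limits, changing the allowed per-frame movement in each direction.
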(event EventBeginPlay
  (bind _returnvalue (UserInterface|CreateWidget "/Game/BluePrints/ScorePanel.ScorePanel_C"))
  (UserInterface|Viewport|AddtoViewport _returnvalue 0))

(event Collision|EventActorBeginOverlap
  (params (OtherActor :type Actor%20Object%20Reference)))

(event EventTick
  (params (DeltaSeconds :type Float%20%28single-precision%29))
  (Transformation|AddLocalOffset (Variables|Default|GetCube) (Math|Vector|MakeVector (Math|Float|Clamp(Float) (* (Class|Actor|GetInputAxisKeyValue) 1e+01) (Variables|Default|GetMinValue) (Variables|Default|GetMax%20Value)) 0.0 0.0) false false))

(fn ConstructionScript)

(fn ChangingSpeed
  (params (MinValue :type Float%20%28single-precision%29) (Max%20Value :type Float%20%28single-precision%29))
  (Variables|Default|SetMinValue MinValue)
  (Variables|Default|SetMax%20Value Max%20Value))